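; Shield pickup item that bobs and spins in place until hit, then plays a pickup sound and destroys itself.
; Each Tick, CalculateHeight turns a wrapping timer into a scaled sine value, which Move adds to the mesh as a local Z offset alongside a fixed rotation step, both per frame.
; The Hit flag is only read here, and no shield effect is applied in this Blueprint.
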(event `self.ReceiveBeginPlay`)

(event `self.ReceiveActorBeginOverlap`
  (params (OtherActor :type "Actor Object Reference")))

(event `self.ReceiveTick`
  (params (DeltaSeconds :type "Float (single-precision)"))
  (if (== (`self.Hit`) true)
    (`GameplayStatics.PlaySoundAtLocation` "/Game/PickUpItem_Cue.PickUpItem_Cue" (`self.K2_GetActorLocation`) (struct) 0.5)
    (`self.K2_DestroyActor`)
    (else
      (bind _height (`self.CalculateHeight` DeltaSeconds))
      (set `self.height` _height)
      (`self.Move`))))

(fn `CalculateHeight`
  (params (deltaT :type "Float (double-precision)"))
  (returns (height :type "Float (double-precision)"))
  (bind _output_get (set `self.t` (+ (`self.t`) deltaT)))
  (if (>= _output_get (`KismetMathLibrary.MultiplyByPi` 2.0))
    (set `self.t` 0.0))
  (return (* (`self.heightScale`) (`KismetMathLibrary.Sin` (`self.t`)))))

(fn `Move`
  (`SceneComponent.K2_AddLocalTransform` (`self.Mesh`) (`KismetMathLibrary.Conv_VectorToTransform` (`KismetMathLibrary.MakeVector` 0.0 0.0 (`self.height`))) false false)
  (`SceneComponent.K2_AddLocalRotation` (`self.Mesh`) (`self.rotation`) false false))

(fn `UserConstructionScript`)