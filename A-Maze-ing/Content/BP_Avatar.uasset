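; BP_Avatar is the player avatar Blueprint, handling HUD setup, the pause menu, death, spell audio and the win flag.
; BeginPlay adds the MHUD widget, and M shows a cached PauseMenu with UI-only input while calling SetGamePaused(false), so play continues.
; Tick polls three functions: zero Hp reopens level Main, five collected items set Win, and the CastSpell flag triggers a one-shot sound before clearing.
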(event `self.ReceiveActorBeginOverlap`
  (params (OtherActor :type "Actor Object Reference")))

(event `self.ReceiveBeginPlay`
  (bind _returnvalue (`|CreateWidget` "/Game/MHUD.MHUD_C"))
  (bind _output_get (set `self.HUD Reference` _returnvalue))
  (`UserWidget.AddToViewport` _output_get 0)
  (`WidgetBlueprintLibrary.SetInputMode_GameOnly` (`GameplayStatics.GetPlayerController` 0)))

(event `Key|M`
  (params (Key :type "Key Structure" :default "AnyKey"))
  (bind _pause_menu_reference (`self.Pause Menu Reference`))
  (:`Pressed`
    (`/Engine/EditorBlueprintResources/StandardMacros.IsValid` (`self.Pause Menu Reference`)
      (:`Is Valid`
        _)
      (:`Is Not Valid`
        (bind _returnvalue (`|CreateWidget` "/Game/PauseMenu.PauseMenu_C"))
        (set `self.Pause Menu Reference` _returnvalue)))
    (`WidgetBlueprintLibrary.SetInputMode_UIOnlyEx` (`GameplayStatics.GetPlayerController` 0) _pause_menu_reference)
    (`UserWidget.AddToViewport` _pause_menu_reference 0)
    (`GameplayStatics.SetGamePaused` false)))

(event `self.ReceiveTick`
  (params (DeltaSeconds :type "Float (single-precision)"))
  (`self.Death`)
  (`self.SpellSound`)
  (`self.CollectedItems`))

(fn `CollectedItems`
  (if (>= (`self.numOfItems`) 5)
    (set `self.Win` true)))

(fn `Death`
  (if (<= (`self.Hp`) 0.0)
    (`GameplayStatics.OpenLevel` "Main")))

(fn `SpellSound`
  (if (== (`self.castSpell`) true)
    (`GameplayStatics.PlaySoundAtLocation` "/Game/Spell_Cue.Spell_Cue" (`self.K2_GetActorLocation`) (struct) 0.5)
    (set `self.castSpell` false)))

(fn `UserConstructionScript`)